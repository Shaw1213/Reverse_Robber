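; BP_Cop is an AI cop that wanders the navmesh, chases pawns it sees and triggers game over on contact.
; Wandering repeats random-point moves; PawnSensing starts a chase, with a once-per-sighting shout and sprint.
; A retriggerable delay after the last sighting slows the cop, rearms the sprint and resumes wandering.
; Any actor overlap shows the player controller's GameOver widget, removed when overlap ends.
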(event OnSeePawn(PawnSensing)
  (params (Pawn :type Pawn%20Object%20Reference))
  ;[1 1 1] AI Pathing
  (Utilities|FlowControl|Sequence
    (:then_0
      (Utilities|FlowControl|DoOnce false
        (:Completed
          (Audio|PlaySound2D "/Game/Brycen_Test/Sounds/Hey__Sound.Hey__Sound" 1.0 1.0 0.0 0 0)
          (Components|Animation|PlayAnimation (Variables|Character|GetMesh) "/Game/Brycen_Test/Running_Anim_mixamo_com.Running_Anim_mixamo_com" true)
          (Variables|/Script/Engine.CharacterMovementComponent|SetMaxWalkSpeed (Variables|Character|GetCharacterMovement) 4.5e+02))))
    (:then_1
      (AI|AIMoveTo self "0, 0, 0" Pawn 5.0 false
        (:then
          (Utilities|FlowControl|RetriggerableDelay 2.0)
          (Components|Animation|PlayAnimation (Variables|Character|GetMesh) "/Game/Brycen_Test/Running_Anim_mixamo_com.Running_Anim_mixamo_com" true)
          (Variables|/Script/Engine.CharacterMovementComponent|SetMaxWalkSpeed (Variables|Character|GetCharacterMovement) 1.5e+02)
          (CallFunction|CanSrpintAgain)
          (CallFunction|MovetoRandomLoc))))))

(event Custom|MoveToRandomLoc
  ;[1 1 1] AI Pathing
  (bind _randomlocation (Class|NavigationSystemV1|GetRandomLocationinNavigableRadius (Transformation|GetActorLocation) 1e+03 0 0))
  (AI|AIMoveTo self _randomlocation 0 5.0 false
    (:OnSuccess
      (CallFunction|MovetoRandomLoc))))

(event Custom|CanSrpintAgain
  ;[1 1 1] AI Pathing
  (Utilities|FlowControl|DoOnce false) ; enters at Reset
)

(event Collision|EventActorEndOverlap
  (params (OtherActor :type Actor%20Object%20Reference))
  ;[1 1 1] AI_GameOver
  (Variables|Default|SetIs_Collision false)
  (bind _asbp_player_controller (Utilities|Casting|CastToBP_PlayerController (Game|GetPlayerController 0)))
  (Widget|RemovefromParent (Variables|/Game/YaZhou_Test/BP/BP_PlayerController.BP_PlayerController_C|GetGameOver _asbp_player_controller)))

(event EventBeginPlay
  ;[1 1 1] AI Pathing
  (CallFunction|MovetoRandomLoc))

(event Collision|EventActorBeginOverlap
  (params (OtherActor :type Actor%20Object%20Reference))
  ;[1 1 1] AI_GameOver
  (Variables|Default|SetIs_Collision true)
  (bind _asbp_player_controller (Utilities|Casting|CastToBP_PlayerController (Game|GetPlayerController 0)))
  (UserInterface|Viewport|AddtoViewport (Variables|/Game/YaZhou_Test/BP/BP_PlayerController.BP_PlayerController_C|GetGameOver _asbp_player_controller) 0))

(fn ConstructionScript)