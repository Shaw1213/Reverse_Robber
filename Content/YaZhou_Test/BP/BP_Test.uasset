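; BP_Test is a test interactable actor whose Cube slides along its local Y axis in response to the player controller's F-button event.
; Overlap begin and end toggle a collision flag and show or remove the controller's interaction widget, with begin also binding the F event.
; F plays a Timeline driving the lerped offset while overlapping, or reverses it from the end otherwise, as the binding is never removed here.
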(event Custom|F_Button_Event
  (if (Variables|Default|GetIs_Collision)
    (bind _alpha (Timeline|Timeline Play)
      (:Update
        (Transformation|SetRelativeLocation (Variables|Default|GetCube) (Math|Vector|MakeVector 0.0 (Math|Float|Lerp 0.0 4e+01 _alpha) 0.0) false false)))
    (else
      (Timeline|Timeline ReverseFromEnd))))

(event EventBeginPlay)

(event Collision|EventActorEndOverlap
  (params (OtherActor :type Actor%20Object%20Reference))
  (Variables|Default|SetIs_Collision false)
  (bind _asbp_player_controller (Utilities|Casting|CastToBP_PlayerController (Game|GetPlayerController 0)))
  (Widget|RemovefromParent (Variables|/Game/YaZhou_Test/BP/BP_PlayerController.BP_PlayerController_C|GetUIBP_interaction _asbp_player_controller)))

(event EventTick
  (params (DeltaSeconds :type Float%20%28single-precision%29)))

(event Collision|EventActorBeginOverlap
  (params (OtherActor :type Actor%20Object%20Reference))
  (Variables|Default|SetIs_Collision true)
  (bind _asbp_player_controller (Utilities|Casting|CastToBP_PlayerController (Game|GetPlayerController 0)))
  (UserInterface|Viewport|AddtoViewport (Variables|/Game/YaZhou_Test/BP/BP_PlayerController.BP_PlayerController_C|GetUIBP_interaction _asbp_player_controller) 0)
  (EventDispatchers|BindEventtoFButton _asbp_player_controller (delegate Custom|F_Button_Event)))

(fn ConstructionScript)